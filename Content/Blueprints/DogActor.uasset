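; Dog actor with separate body and shadow visuals that reacts visually to being hit by the yoyo.
; Each tick, both visuals take their world Y as translucent sort priority for depth ordering.
; An overlap from a component named yoyo_collider, matched by name string, starts a timeline that blinks the body visual.
; A flag blocks retriggering until the timeline finishes and restores visibility; no health is changed here.
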(event `self.ReceiveBeginPlay`)

(event `self.ReceiveTick`
  (params (DeltaSeconds :type "Float (single-precision)"))
  (`self.fixTranslucentPriority`))

(event `self.ReceiveActorBeginOverlap`
  (params (OtherActor :type "Actor Object Reference")))

(event `self.dog_collider.OnComponentBeginOverlap`
  (params (OtherActor :type "Actor Object Reference") (OtherComp :type "PrimitiveComponent Object Reference") (OtherBodyIndex :type Integer) (bFromSweep :type Boolean) (SweepResult :type "HitResult Structure (by ref)"))
  (bind _returnvalue (`KismetSystemLibrary.GetObjectName` OtherComp))
  (`KismetSystemLibrary.PrintString` _returnvalue true true (struct :`R` 1.0 :`B` 0.8476 :`A` 1.0))
  (if (and (`KismetStringLibrary.EqualEqual_StrStr` _returnvalue "yoyo_collider") (not (`self.isShowingDamage`)))
    (set `self.isShowingDamage` true)
    (bind (_direction _newtrack_3) (`Timeline|Timeline_0` :!via `PlayFromStart`)
      (:`Update`
        (if (<= (mod _newtrack_3 2.0) 1.0)
          (`SceneComponent.SetVisibility` (`self.dog_visual`) false false)
          (else
            (`SceneComponent.SetVisibility` (`self.dog_visual`) true false :!label _label))))
      (:`Finished`
        (set `self.isShowingDamage` false)
        (goto _label)))))

(fn `fixTranslucentPriority`
  (bind _dog_visual (`self.dog_visual`))
  (bind _shadow_visual (`self.shadow_visual`))
  (`PrimitiveComponent.SetTranslucentSortPriority` _dog_visual (`KismetMathLibrary.FTrunc` (.y (`SceneComponent.K2_GetComponentLocation` _dog_visual))))
  (`PrimitiveComponent.SetTranslucentSortPriority` _shadow_visual (`KismetMathLibrary.FTrunc` (.y (`SceneComponent.K2_GetComponentLocation` _shadow_visual)))))

(fn `UserConstructionScript`)