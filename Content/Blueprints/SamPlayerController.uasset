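; Player controller for SamPawnBlueprint that handles movement on X and Z, jumping, and a yoyo attack.
; Axis inputs feed movement input, while Tick sets the pawn's Y to minus half its Z, tying depth to height.
; Jump and Attack use timelines to offset only the Sam and yoyo visuals, with flags blocking retriggers.
; The yoyo is shown only during the attack.
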(event `self.ReceiveBeginPlay`)

(event `self.ReceiveTick`
  (params (DeltaSeconds :type "Float (single-precision)"))
  (`self.adjustYPosition`))

(event `InputAxis|Right`
  (params (AxisValue :type "Float (single-precision)"))
  (`self.moveHorizontal` AxisValue))

(event `InputAxis|Up`
  (params (AxisValue :type "Float (single-precision)"))
  (`self.moveVertical` AxisValue))

(event `InputAction|Jump`
  (params (Key :type "Key Structure" :default "AnyKey"))
  (:`Pressed`
    (if (not (`self.isJumping`))
      (set `self.isJumping` true)
      (bind _assam_pawn_blueprint (cast `/Game/Blueprints/SamPawnBlueprint` (`self.K2_GetPawn`)))
      (bind (_direction _newtrack_1) (`Timeline|JumpTimeline` :!via `PlayFromStart`)
        (:`Update`
          (`SceneComponent.K2_SetRelativeLocation` (`/Game/Blueprints/SamPawnBlueprint.sam_visual` _assam_pawn_blueprint) (`KismetMathLibrary.MakeVector` 0.0 0.0 (* _newtrack_1 300.0)) false false))
        (:`Finished`
          (set `self.isJumping` false))))))

(event `InputAction|Attack`
  (params (Key :type "Key Structure" :default "AnyKey"))
  (:`Pressed`
    (if (not (`self.isAttacking`))
      (set `self.isAttacking` true)
      (bind _assam_pawn_blueprint (cast `/Game/Blueprints/SamPawnBlueprint` (`self.K2_GetPawn`)))
      (bind _yoyo_visual (`/Game/Blueprints/SamPawnBlueprint.yoyo_visual` _assam_pawn_blueprint))
      (`SceneComponent.SetVisibility` _yoyo_visual true false)
      (bind (_direction _newtrack_2) (`Timeline|AttackTimeline` :!via `PlayFromStart`)
        (:`Update`
          (`SceneComponent.K2_SetRelativeLocation` _yoyo_visual (`KismetMathLibrary.MakeVector` (* _newtrack_2 200.0)) false false))
        (:`Finished`
          (set `self.isAttacking` false)
          (`SceneComponent.SetVisibility` _yoyo_visual false false))))))

(fn `adjustYPosition`
  (bind _returnvalue (`self.K2_GetPawn`))
  (bind _z (.z (`self.K2_GetActorLocation` _returnvalue)))
  (`self.K2_SetActorLocation` _returnvalue (`KismetMathLibrary.MakeVector` (.x (`self.K2_GetActorLocation` _returnvalue)) (/ _z -2.0) _z) false false))

(fn `jump`)

(fn `moveHorizontal`
  (params (value :type "Float (double-precision)"))
  (`Pawn.AddMovementInput` (`self.K2_GetPawn`) (`KismetMathLibrary.MakeVector` value) 0.5 false))

(fn `moveVertical`
  (params (value :type "Float (double-precision)"))
  (`Pawn.AddMovementInput` (`self.K2_GetPawn`) (`KismetMathLibrary.MakeVector` 0.0 0.0 value) 0.5 false))

(fn `UserConstructionScript`)