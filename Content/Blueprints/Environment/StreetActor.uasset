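; StreetActor is a street piece that scrolls along X and recycles itself to form a looping road.
; Each Tick it moves by WorldManager's WorldSpeed through a swept InterpToMovement update, without delta-time scaling.
; On passing the negative X limit it jumps to the opposite end, keeping Y, fixing Z and offsetting X by the world speed and its scaled increase.
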(event `self.ReceiveBeginPlay`)

(event `self.ReceiveActorBeginOverlap`
  (params (OtherActor :type "Actor Object Reference")))

(event `self.ReceiveTick`
  (params (DeltaSeconds :type "Float (single-precision)"))
  (bind _worldmanager (`self.WorldManager`))
  (`MovementComponent.K2_MoveUpdatedComponent` :`self` (`self.InterpToMovement`) :`Delta` (`KismetMathLibrary.MakeVector` (`/Game/Blueprints/World_Manager_Blueprint.WorldSpeed` (`self.WorldManager`))))
  (if (<= (.x (`self.K2_GetActorLocation`)) -1920.0)
    (`self.K2_SetActorLocation` self (`KismetMathLibrary.MakeVector` (+ (+ 1920.0 (`/Game/Blueprints/World_Manager_Blueprint.WorldSpeed` _worldmanager)) (* (`/Game/Blueprints/World_Manager_Blueprint.worldSpeedIncrease` _worldmanager) 10.0)) (.y (`self.K2_GetActorLocation`)) -20.0) false false)))

(fn `UserConstructionScript`)