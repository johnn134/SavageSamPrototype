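; Player pawn for Sam: creates the HUD and handles scoring, pickups, yoyo hits, skateboard ramp jumps and bus game over.
; Separate body and shadow colliders fake depth: some obstacles hit only when both overlap the same actor, static ones by shadow alone.
; Damage flashes Sam, removes the skateboard and resets World Manager speed, which soda boosts.
; Timelines drive jumps, flashes and Pow/Yeah popups; Tick sorts sprites by world Y.
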(event `self.ReceiveBeginPlay`
  ;[1 1 1] Initialize visibilities
  (`SceneComponent.SetVisibility` (`self.yoyo_visual`) false false)
  (`SceneComponent.SetVisibility` (`self.skateboard_visual`) false false)
  ;[1 1 1] Turn off collisions on yoyo
  (set `PrimitiveComponent.bGenerateOverlapEvents` false (`self.yoyo_collider`))
  ;[1 1 1] Create Game HUD
  (bind _returnvalue (`|CreateWidget` "/Game/GUI/SavageSamHUD.SavageSamHUD_C"))
  (bind _output_get (set `self.HUDReference` _returnvalue))
  (`UserWidget.AddToViewport` _output_get 0)
  (`WidgetBlueprintLibrary.SetInputMode_GameOnly` (`GameplayStatics.GetPlayerController` 0))
  ;[1 1 1] Find Popup objects
  (bind _outactors (`GameplayStatics.GetAllActorsOfClass` "/Game/Blueprints/Popups/PowActor.PowActor_C"))
  (set `self.pow_ref` (`KismetArrayLibrary.Array_Get` _outactors))
  (bind _outactors_2 (`GameplayStatics.GetAllActorsOfClass` "/Game/Blueprints/Popups/YeahActor.YeahActor_C"))
  (set `self.yeah_ref` (`KismetArrayLibrary.Array_Get` _outactors_2))
  ;[1 1 1] Find and grab values from the world manager
  (bind _outactors_3 (`GameplayStatics.GetAllActorsOfClass` "/Game/Blueprints/World_Manager_Blueprint.World_Manager_Blueprint_C"))
  (bind _output_get_2 (set `self.WorldManager` (`KismetArrayLibrary.Array_Get` _outactors_3)))
  (set `self.defaultWorldSpeed` (`/Game/Blueprints/World_Manager_Blueprint.WorldSpeed` _output_get_2)))

(event `self.ReceiveTick`
  (params (DeltaSeconds :type "Float (single-precision)"))
  (`self.fixTranslucentPriority`))

(event `self.sam_collider.OnComponentBeginOverlap`
  (params (OtherActor :type "Actor Object Reference") (OtherComp :type "PrimitiveComponent Object Reference") (OtherBodyIndex :type Integer) (bFromSweep :type Boolean) (SweepResult :type "HitResult Structure (by ref)"))
  (bind _worldmanager (`self.WorldManager`))
  (bind _visualoverlapactor (`self.visualOverlapActor`))
  (set `self.isOverlappingVisual` true)
  (set `self.visualOverlapActor` OtherActor)
  (set `self.visualOverlapComponent` OtherComp)
  ;[1 1 1] Pickup Collision Check
  (bind _returnvalue (`PrimitiveComponent.GetCollisionProfileName` (`self.visualOverlapComponent`)))
  (if (== _returnvalue "PickupVisual")
    ;[1 1 1] Case handling for different pickups
    (cast `/Game/Blueprints/Pickups/SodaActor` _visualoverlapactor
      (:`then`
        (set `/Game/Blueprints/World_Manager_Blueprint.WorldSpeed` (+ (`/Game/Blueprints/World_Manager_Blueprint.WorldSpeed` _worldmanager) (`self.sodaSpeedBuff`)) _worldmanager)
        (set `self.score` (+ (`self.score`) (`self.sodaPoints`))))
      (:`CastFailed`
        (cast `/Game/Blueprints/Pickups/PizzaActor` _visualoverlapactor
          (:`then`
            (set `self.score` (+ (`self.score`) (`self.PizzaPoints`))))
          (:`CastFailed`
            (cast `/Game/Blueprints/Pickups/SkateboardActor` _visualoverlapactor)
            (set `self.isSkateboarding` true)
            (bind _assam_player_controller (cast `/Game/Blueprints/MainCharacter/SamPlayerController` (`GameplayStatics.GetPlayerController` 0)))
            (set `/Game/Blueprints/MainCharacter/SamPlayerController.isSkateboarding` true _assam_player_controller)
            (`SceneComponent.SetVisibility` (`self.skateboard_visual`) true false)
            (set `self.score` (+ (`self.score`) (`self.skateboardPoints`)))))))
    ;[1 1 1] Yeah Popup from pickups
    (`self.K2_SetActorLocation` (`self.yeah_ref`) (+ (`self.K2_GetActorLocation`) (`self.yeahOffset`)) false false :!label _label)
    (`Timeline|Timeline_1` :!via `PlayFromStart`
      (:`Finished`
        (`self.K2_SetActorLocation` (`self.yeah_ref`) (0.0 0.0 1000.0) false false)))))

(event `self.shadow_collider.OnComponentBeginOverlap`
  (params (OtherActor :type "Actor Object Reference") (OtherComp :type "PrimitiveComponent Object Reference") (OtherBodyIndex :type Integer) (bFromSweep :type Boolean) (SweepResult :type "HitResult Structure (by ref)"))
  (set `self.isOverlappingShadow` true)
  (set `self.shadowOverlapActor` OtherActor)
  (set `self.shadowOverlapComponent` OtherComp)
  ;[1 1 1] Check for Bus Collision
  (cast `/Game/Blueprints/Obstacles/BusActor` (`self.visualOverlapActor`)
    (:`then`
      (`/Game/Blueprints/World_Manager_Blueprint.endGame` (`self.WorldManager`) (`self.score`)))
    (:`CastFailed`
      ;[1 1 1] Check for Ramp Collision While Skateboarding
      (bind _returnvalue (`PrimitiveComponent.GetCollisionProfileName` (`self.shadowOverlapComponent`)))
      (if (and (== _returnvalue "Ramp") (`self.isSkateboarding`))
        (set `self.score` (+ (`self.score`) (`self.rampPoints`)))
        ;[1 1 1] Begin Ramp Jump
        (bind _assam_player_controller (cast `/Game/Blueprints/MainCharacter/SamPlayerController` (`GameplayStatics.GetPlayerController` 0)))
        (if (not (`/Game/Blueprints/MainCharacter/SamPlayerController.isJumping` _assam_player_controller))
          (set `/Game/Blueprints/MainCharacter/SamPlayerController.isJumping` true _assam_player_controller)
          (bind (_direction _newtrack_1) (`Timeline|Timeline_3` :!via `PlayFromStart`)
            (:`Update`
              (bind _returnvalue_2 (* _newtrack_1 (`self.rampJumpHeight`)))
              (`SceneComponent.K2_SetRelativeLocation` (`self.sam_visual`) (`KismetMathLibrary.MakeVector` 0.0 0.0 (+ _returnvalue_2 135.0)) false false)
              (`SceneComponent.K2_SetRelativeLocation` (`self.skateboard_visual`) (`KismetMathLibrary.MakeVector` 0.0 0.0 (- _returnvalue_2 10.0)) false false)
              (if (not (`self.rampJumpStarted`))
                (set `self.rampJumpStarted` true)
                (goto _label)))
            (:`Finished`
              (set `/Game/Blueprints/MainCharacter/SamPlayerController.isJumping` false _assam_player_controller)
              (set `self.rampJumpStarted` false))))
        (else
          ;[1 1 1] Ignore ramp if skateboarding
          (cast `/Game/Blueprints/Obstacles/RampActor` (`self.shadowOverlapActor`)
            (:`then`
              (if (not (`self.isSkateboarding`))
                ;[1 1 1] Static Obstacle Collision Check
                (bind _returnvalue_3 (`PrimitiveComponent.GetCollisionProfileName` (`self.shadowOverlapComponent`) :!label _label_2))
                (if (and (== _returnvalue_3 "ObstacleStatic") (not (`self.isShowingDamage`)))
                  ;[1 1 1] Remove Skateboard buff when damaged
                  (set `self.isSkateboarding` false :!label _label_3)
                  (bind _assam_player_controller_2 (cast `/Game/Blueprints/MainCharacter/SamPlayerController` (`GameplayStatics.GetPlayerController` 0)))
                  (set `/Game/Blueprints/MainCharacter/SamPlayerController.isSkateboarding` false _assam_player_controller_2)
                  (`SceneComponent.SetVisibility` (`self.skateboard_visual`) false false)
                  ;[1 1 1] Reset world speed when hit
                  (set `/Game/Blueprints/World_Manager_Blueprint.WorldSpeed` (`self.defaultWorldSpeed`) (`self.WorldManager`))
                  ;[1 1 1] Damage Flash
                  (set `self.isShowingDamage` true)
                  (bind (_direction_2 _newtrack_4) (`Timeline|Timeline_0` :!via `PlayFromStart`)
                    (:`Update`
                      (if (<= (mod _newtrack_4 2.0) 1.0)
                        (`SceneComponent.SetVisibility` (`self.sam_visual`) false false)
                        (else
                          (`SceneComponent.SetVisibility` (`self.sam_visual`) true false :!label _label_4))))
                    (:`Finished`
                      (set `self.isShowingDamage` false)
                      (goto _label_4)))
                  (else
                    ;[1 1 1] Obstacle Collision Check
                    (if (and (`self.isOverlappingVisual`) (`self.isOverlappingShadow`))
                      (bind _returnvalue_4 (`PrimitiveComponent.GetCollisionProfileName` (`self.visualOverlapComponent`)))
                      (bind _returnvalue_5 (`PrimitiveComponent.GetCollisionProfileName` (`self.shadowOverlapComponent`)))
                      (if (and (and (and (== _returnvalue_5 "ObstacleShadow") (== _returnvalue_4 "ObstacleVisual")) (== (`self.visualOverlapActor`) (`self.shadowOverlapActor`))) (not (`self.isShowingDamage`)))
                        (goto _label_3)))))))
            (:`CastFailed`
              (goto _label_2))))))))

(event `self.shadow_collider.OnComponentEndOverlap`
  (params (OtherActor :type "Actor Object Reference") (OtherComp :type "PrimitiveComponent Object Reference") (OtherBodyIndex :type Integer))
  (set `self.isOverlappingShadow` false)
  (set `self.shadowOverlapActor` null)
  (set `self.shadowOverlapComponent` null))

(event `self.sam_collider.OnComponentEndOverlap`
  (params (OtherActor :type "Actor Object Reference") (OtherComp :type "PrimitiveComponent Object Reference") (OtherBodyIndex :type Integer))
  (set `self.isOverlappingVisual` false)
  (set `self.visualOverlapActor` null)
  (set `self.visualOverlapComponent` null))

(event `self.yoyo_collider.OnComponentBeginOverlap`
  (params (OtherActor :type "Actor Object Reference") (OtherComp :type "PrimitiveComponent Object Reference") (OtherBodyIndex :type Integer) (bFromSweep :type Boolean) (SweepResult :type "HitResult Structure (by ref)"))
  (set `self.score` (+ (`self.score`) (`self.attackPoints`)))
  ;[1 1 1] Place Pow Sprite on yoyo collision
  (`self.K2_SetActorLocation` (`self.pow_ref`) (+ (`SceneComponent.K2_GetComponentLocation` (`self.yoyo_visual`)) (`self.powOffset`)) false false)
  (`Timeline|Timeline_2` :!via `PlayFromStart`
    (:`Finished`
      (`self.K2_SetActorLocation` (`self.pow_ref`) (0.0 0.0 1000.0) false false))))

(fn `fixTranslucentPriority`
  (bind _yoyo_visual (`self.yoyo_visual`))
  (bind _sam_visual (`self.sam_visual`))
  (bind _shadow_visual (`self.shadow_visual`))
  (`PrimitiveComponent.SetTranslucentSortPriority` _sam_visual (`KismetMathLibrary.FTrunc` (.y (`SceneComponent.K2_GetComponentLocation` _sam_visual))))
  (`PrimitiveComponent.SetTranslucentSortPriority` _shadow_visual (`KismetMathLibrary.FTrunc` (.y (`SceneComponent.K2_GetComponentLocation` _shadow_visual))))
  (`PrimitiveComponent.SetTranslucentSortPriority` _yoyo_visual (`KismetMathLibrary.FTrunc` (.y (`SceneComponent.K2_GetComponentLocation` _yoyo_visual)))))

(fn `UserConstructionScript`)