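; Pawn for the character Sam, with sprite depth sorting, damage flicker and a yoyo that starts hidden.
; Every tick, the Sam, shadow and yoyo visuals take their translucent sort priority from their world Y position.
; Overlapping a GameObstacle profile starts a timeline that blinks Sam's visual, with a flag blocking retriggers until it finishes.
; Yoyo collider overlaps only print a debug message.
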(event `self.ReceiveBeginPlay`
  (`SceneComponent.SetVisibility` (`self.yoyo_visual`) false false))

(event `self.ReceiveActorBeginOverlap`
  (params (OtherActor :type "Actor Object Reference")))

(event `self.ReceiveTick`
  (params (DeltaSeconds :type "Float (single-precision)"))
  (`self.fixTranslucentPriority`))

(event `self.yoyo_collider.OnComponentBeginOverlap`
  (params (OtherActor :type "Actor Object Reference") (OtherComp :type "PrimitiveComponent Object Reference") (OtherBodyIndex :type Integer) (bFromSweep :type Boolean) (SweepResult :type "HitResult Structure (by ref)"))
  (`KismetSystemLibrary.PrintString` (`KismetStringLibrary.Concat_StrStr` "Yoyo collided with " (`KismetSystemLibrary.GetDisplayName` OtherComp))))

(event `self.sam_collider.OnComponentBeginOverlap`
  (params (OtherActor :type "Actor Object Reference") (OtherComp :type "PrimitiveComponent Object Reference") (OtherBodyIndex :type Integer) (bFromSweep :type Boolean) (SweepResult :type "HitResult Structure (by ref)"))
  (bind _returnvalue (`PrimitiveComponent.GetCollisionProfileName` OtherComp))
  (if (and (== _returnvalue "GameObstacle") (not (`self.isShowingDamage`)))
    (set `self.isShowingDamage` true)
    (bind (_direction _newtrack_4) (`Timeline|Timeline_0` :!via `PlayFromStart`)
      (:`Update`
        (if (<= (mod _newtrack_4 2.0) 1.0)
          (`SceneComponent.SetVisibility` (`self.sam_visual`) false false)
          (else
            (`SceneComponent.SetVisibility` (`self.sam_visual`) true false :!label _label))))
      (:`Finished`
        (set `self.isShowingDamage` false)
        (goto _label)))))

(fn `fixTranslucentPriority`
  (bind _yoyo_visual (`self.yoyo_visual`))
  (bind _sam_visual (`self.sam_visual`))
  (bind _shadow_visual (`self.shadow_visual`))
  (`PrimitiveComponent.SetTranslucentSortPriority` _sam_visual (`KismetMathLibrary.FTrunc` (.y (`SceneComponent.K2_GetComponentLocation` _sam_visual))))
  (`PrimitiveComponent.SetTranslucentSortPriority` _shadow_visual (`KismetMathLibrary.FTrunc` (.y (`SceneComponent.K2_GetComponentLocation` _shadow_visual))))
  (`PrimitiveComponent.SetTranslucentSortPriority` _yoyo_visual (`KismetMathLibrary.FTrunc` (.y (`SceneComponent.K2_GetComponentLocation` _yoyo_visual)))))

(fn `UserConstructionScript`)