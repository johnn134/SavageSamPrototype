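; StreetHouseActor is a scrolling street-and-houses backdrop piece that moves steadily along negative X to fake travel.
; Each tick it moves via its InterpToMovement component with a fixed delta, then jumps back to the right edge once it passes the left limit, forming a loop.
; It also re-sets the translucent sort priority of its street and house visuals from their world Y, so layers draw in depth order.
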(event `self.ReceiveBeginPlay`)

(event `self.ReceiveActorBeginOverlap`
  (params (OtherActor :type "Actor Object Reference")))

(event `self.ReceiveTick`
  (params (DeltaSeconds :type "Float (single-precision)"))
  (`self.fixTranslucentPriority`)
  (`MovementComponent.K2_MoveUpdatedComponent` :`self` (`self.InterpToMovement`) :`Delta` (-2.0 0.0 0.0))
  (if (<= (.x (`self.K2_GetActorLocation`)) -1920.0)
    (`self.K2_SetActorLocation` self (`KismetMathLibrary.MakeVector` 1920.0 -400.0) false false)))

(fn `fixTranslucentPriority`
  (bind _street_visual (`self.street_visual`))
  (bind _houses_visual (`self.houses_visual`))
  (`PrimitiveComponent.SetTranslucentSortPriority` _street_visual (`KismetMathLibrary.FTrunc` (.y (`SceneComponent.K2_GetComponentLocation` _street_visual))))
  (`PrimitiveComponent.SetTranslucentSortPriority` _houses_visual (`KismetMathLibrary.FTrunc` (.y (`SceneComponent.K2_GetComponentLocation` _houses_visual)))))

(fn `UserConstructionScript`)