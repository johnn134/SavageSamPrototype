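; Soda pickup actor that scrolls along X at the World Manager's speed, taking the manager from its owner if unset.
; Each tick it derives Y from height (-Z/2) and sets visual and shadow translucent sort priority from world Y to layer them by depth.
; While movable it sweeps by a per-frame step unscaled by delta time, and a replayed timeline bobs the visual vertically.
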(event `self.ReceiveBeginPlay`
  ;[1 1 1] Set World Manager to Owner if not already assigned
  (if (not (!= (`self.WorldManager`) null))
    (bind _asworld_manager_blueprint (cast `/Game/Blueprints/World_Manager_Blueprint` (`self.GetOwner`)))
    (set `self.WorldManager` _asworld_manager_blueprint)))

(event `self.ReceiveActorBeginOverlap`
  (params (OtherActor :type "Actor Object Reference")))

(event `self.ReceiveTick`
  (params (DeltaSeconds :type "Float (single-precision)"))
  (`self.fixTranslucentPriority`)
  (`self.adjustYPosition`)
  ;[1 1 1] Movement
  (if (`self.canMove`)
    (`MovementComponent.K2_MoveUpdatedComponent` :`self` (`self.InterpToMovement`) :`Delta` (`KismetMathLibrary.MakeVector` (`/Game/Blueprints/World_Manager_Blueprint.WorldSpeed` (`self.WorldManager`)))))
  ;[1 1 1] Pickup floating
  (if (not (`self.floating`))
    (set `self.floating` true)
    (bind (_direction _newtrack_0) (`Timeline|Timeline_0` :!via `PlayFromStart`)
      (:`Update`
        (`SceneComponent.K2_SetRelativeLocation` (`self.pickup_visual`) (`KismetMathLibrary.MakeVector` 0.0 0.0 (* _newtrack_0 10.0)) false false))
      (:`Finished`
        (set `self.floating` false)))))

(fn `adjustYPosition`
  (bind _z (.z (`self.K2_GetActorLocation`)))
  (`self.K2_SetActorLocation` (`KismetMathLibrary.MakeVector` (.x (`self.K2_GetActorLocation`)) (/ _z -2.0) _z)))

(fn `fixTranslucentPriority`
  (bind _pickup_visual (`self.pickup_visual`))
  (bind _pickup_shadow (`self.pickup_shadow`))
  (`PrimitiveComponent.SetTranslucentSortPriority` _pickup_visual (`KismetMathLibrary.FTrunc` (.y (`SceneComponent.K2_GetComponentLocation` _pickup_visual))))
  (`PrimitiveComponent.SetTranslucentSortPriority` _pickup_shadow (`KismetMathLibrary.FTrunc` (.y (`SceneComponent.K2_GetComponentLocation` _pickup_shadow)))))

(fn `UserConstructionScript`)