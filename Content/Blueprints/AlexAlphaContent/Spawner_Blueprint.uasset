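; Spawner Blueprint that procedurally lays out a random obstacle course along the X axis, generated in full at BeginPlay.
; A loop steps CurrentX toward a fixed end distance, randomly deciding at each step whether to spawn one of four obstacle classes at a random height, owned by WorldManagerRef.
; After each spawn, MakeBuffer advances CurrentX by that obstacle type's buffer distance to space out the next one.
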(event `self.ReceiveBeginPlay`
  (bind _currentx (`self.CurrentX`))
  (bind _obsticalid (`self.ObsticalID`))
  (while (>= 150000 _currentx)
    (set `self.CurrentX` (+ _currentx 1))
    (if (== (`KismetMathLibrary.RandomIntegerInRange` 0 10) 5)
      (set `self.ObsticalID` (`KismetMathLibrary.RandomIntegerInRange` 0 3))
      (`|SpawnActorFromClass` (`KismetArrayLibrary.Array_Get` (`self.ObsticalClasses`) _obsticalid) (`KismetMathLibrary.MakeTransform` (`KismetMathLibrary.MakeVector` (`KismetMathLibrary.Conv_IntToDouble` _currentx) 0.0 (`KismetMathLibrary.RandomFloatInRange` -300.0 175.0))) "Undefined" "OverrideRootScale" (`self.WorldManagerRef`))
      (`self.MakeBuffer` _obsticalid))))

(fn `MakeBuffer`
  (params (ObsticalID :type Integer))
  (set `self.CurrentX` (+ (`KismetArrayLibrary.Array_Get` (`self.BufferDistances`) ObsticalID) (`self.CurrentX`))))

(fn `UserConstructionScript`)