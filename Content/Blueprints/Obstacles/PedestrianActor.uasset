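; Pedestrian obstacle that moves along X at the World Manager's WorldSpeed and flashes when hit, using its owner as manager if none is set.
; Each tick fakes depth by deriving Y from Z and setting sprite and shadow translucent sort priority from Y.
; A body hit requires visual and shadow colliders to overlap the same Sam actor, while a yoyo needs only the visual.
; Hits play a timeline that blinks the visual, without applying damage.
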(event `self.ReceiveBeginPlay`
  ;[1 1 1] Set World Manager to Owner if not already assigned
  (if (not (!= (`self.WorldManager`) null))
    (bind _asworld_manager_blueprint (cast `/Game/Blueprints/World_Manager_Blueprint` (`self.GetOwner`)))
    (set `self.WorldManager` _asworld_manager_blueprint)))

(event `self.ReceiveTick`
  (params (DeltaSeconds :type "Float (single-precision)"))
  (`self.fixTranslucentPriority`)
  (`self.adjustYPosition`)
  ;[1 1 1] Movement
  (if (`self.canMove`)
    (`MovementComponent.K2_MoveUpdatedComponent` :`self` (`self.InterpToMovement`) :`Delta` (`KismetMathLibrary.MakeVector` (`/Game/Blueprints/World_Manager_Blueprint.WorldSpeed` (`self.WorldManager`))))))

(event `self.shadow_collider.OnComponentBeginOverlap`
  (params (OtherActor :type "Actor Object Reference") (OtherComp :type "PrimitiveComponent Object Reference") (OtherBodyIndex :type Integer) (bFromSweep :type Boolean) (SweepResult :type "HitResult Structure (by ref)"))
  (set `self.isOverlappingShadow` true)
  (set `self.shadowOverlapActor` OtherActor)
  (set `self.shadowOverlapComponent` OtherComp)
  ;[1 1 1] Body Collision
  (if (and (`self.isOverlappingVisual`) (`self.isOverlappingShadow`)) :!label _label
    (bind _returnvalue (`PrimitiveComponent.GetCollisionProfileName` (`self.visualOverlapComponent`)))
    (bind _returnvalue_2 (`PrimitiveComponent.GetCollisionProfileName` (`self.shadowOverlapComponent`)))
    (if (and (and (and (== _returnvalue_2 "SamShadow") (== _returnvalue "SamVisual")) (== (`self.visualOverlapActor`) (`self.shadowOverlapActor`))) (not (`self.isShowingDamage`)))
      ;[1 1 1] Damage flash
      (set `self.isShowingDamage` true :!label _label_2)
      (bind (_direction _newtrack_3) (`Timeline|Timeline_0` :!via `PlayFromStart`)
        (:`Update`
          (if (<= (mod _newtrack_3 2.0) 1.0)
            (`SceneComponent.SetVisibility` (`self.obstacle_visual`) false false)
            (else
              (`SceneComponent.SetVisibility` (`self.obstacle_visual`) true false :!label _label_3))))
        (:`Finished`
          (set `self.isShowingDamage` false)
          (goto _label_3))))))

(event `self.visual_collider.OnComponentBeginOverlap`
  (params (OtherActor :type "Actor Object Reference") (OtherComp :type "PrimitiveComponent Object Reference") (OtherBodyIndex :type Integer) (bFromSweep :type Boolean) (SweepResult :type "HitResult Structure (by ref)"))
  (set `self.isOverlappingVisual` true)
  (set `self.visualOverlapActor` OtherActor)
  (set `self.visualOverlapComponent` OtherComp)
  ;[1 1 1] Yoyo Collision Check
  (bind _returnvalue (`PrimitiveComponent.GetCollisionProfileName` (`self.visualOverlapComponent`)))
  (if (and (== _returnvalue "yoyo") (not (`self.isShowingDamage`)))
    (goto _label_2)
    (else
      (goto _label))))

(event `self.shadow_collider.OnComponentEndOverlap`
  (params (OtherActor :type "Actor Object Reference") (OtherComp :type "PrimitiveComponent Object Reference") (OtherBodyIndex :type Integer))
  (set `self.isOverlappingShadow` false)
  (set `self.shadowOverlapActor` OtherActor)
  (set `self.shadowOverlapComponent` OtherComp))

(event `self.visual_collider.OnComponentEndOverlap`
  (params (OtherActor :type "Actor Object Reference") (OtherComp :type "PrimitiveComponent Object Reference") (OtherBodyIndex :type Integer))
  (set `self.isOverlappingVisual` false)
  (set `self.visualOverlapActor` OtherActor)
  (set `self.visualOverlapComponent` OtherComp))

(fn `adjustYPosition`
  (bind _z (.z (`self.K2_GetActorLocation`)))
  (`self.K2_SetActorLocation` (`KismetMathLibrary.MakeVector` (.x (`self.K2_GetActorLocation`)) (/ _z -2.0) _z)))

(fn `fixTranslucentPriority`
  (bind _obstacle_visual (`self.obstacle_visual`))
  (bind _shadow_visual (`self.shadow_visual`))
  (`PrimitiveComponent.SetTranslucentSortPriority` _obstacle_visual (`KismetMathLibrary.FTrunc` (.y (`SceneComponent.K2_GetComponentLocation` _obstacle_visual))))
  (`PrimitiveComponent.SetTranslucentSortPriority` _shadow_visual (`KismetMathLibrary.FTrunc` (.y (`SceneComponent.K2_GetComponentLocation` _shadow_visual)))))

(fn `UserConstructionScript`)