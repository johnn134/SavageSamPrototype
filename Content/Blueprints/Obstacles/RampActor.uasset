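; Ramp obstacle actor that scrolls along X at the world manager's WorldSpeed while CanMove is set.
; On BeginPlay it takes the world manager from its owner if none is assigned.
; Each tick it derives Y from height (minus half Z) and sets obstacle and shadow translucent sort priority from world Y to fake depth ordering.
; Movement is a swept per-frame offset through InterpToMovement, not scaled by delta time.
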(event `self.ReceiveBeginPlay`
  ;[1 1 1] Set World Manager to Owner if not already assigned
  (if (not (!= (`self.WorldManager`) null))
    (bind _asworld_manager_blueprint (cast `/Game/Blueprints/World_Manager_Blueprint` (`self.GetOwner`)))
    (set `self.WorldManager` _asworld_manager_blueprint)))

(event `self.ReceiveTick`
  (params (DeltaSeconds :type "Float (single-precision)"))
  (`self.fixTranslucentPriority`)
  (`self.adjustYPosition`)
  ;[1 1 1] Movement
  (if (`self.canMove`)
    (`MovementComponent.K2_MoveUpdatedComponent` :`self` (`self.InterpToMovement`) :`Delta` (`KismetMathLibrary.MakeVector` (`/Game/Blueprints/World_Manager_Blueprint.WorldSpeed` (`self.WorldManager`))))))

(fn `adjustYPosition`
  (bind _z (.z (`self.K2_GetActorLocation`)))
  (`self.K2_SetActorLocation` (`KismetMathLibrary.MakeVector` (.x (`self.K2_GetActorLocation`)) (/ _z -2.0) _z)))

(fn `fixTranslucentPriority`
  (bind _obstacle_visual (`self.obstacle_visual`))
  (bind _shadow_visual (`self.shadow_visual`))
  (`PrimitiveComponent.SetTranslucentSortPriority` _obstacle_visual (`KismetMathLibrary.FTrunc` (.y (`SceneComponent.K2_GetComponentLocation` _obstacle_visual))))
  (`PrimitiveComponent.SetTranslucentSortPriority` _shadow_visual (`KismetMathLibrary.FTrunc` (.y (`SceneComponent.K2_GetComponentLocation` _shadow_visual)))))

(fn `UserConstructionScript`)