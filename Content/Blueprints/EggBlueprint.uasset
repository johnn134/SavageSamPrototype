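; Egg actor that scrolls along negative X as part of a moving world, starting at a random lateral Y offset set on BeginPlay.
; Each Tick it casts its owner to World_Manager_Blueprint and sets the root to the Sphere's location shifted by WorldSpeed, without delta-time scaling.
; It destroys itself once that shifted X drops below zero.
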(event `self.ReceiveBeginPlay`
  (`SceneComponent.K2_SetWorldLocation` (`self.DefaultSceneRoot`) (`KismetMathLibrary.MakeVector` (.x (`self.K2_GetActorLocation`)) (`KismetMathLibrary.RandomFloatInRange` -200.0 200.0) (.z (`self.K2_GetActorLocation`))) false false))

(event `self.ReceiveTick`
  (params (DeltaSeconds :type "Float (single-precision)"))
  (bind _asworld_manager_blueprint (cast `/Game/Blueprints/World_Manager_Blueprint` (`self.GetOwner`)))
  (bind _returnvalue (- (`SceneComponent.K2_GetComponentLocation` (`self.Sphere`)) (`KismetMathLibrary.MakeVector` (`/Game/Blueprints/World_Manager_Blueprint.WorldSpeed` _asworld_manager_blueprint))))
  (`SceneComponent.K2_SetWorldLocation` (`self.DefaultSceneRoot`) _returnvalue false false)
  (if (> 0.0 (.x _returnvalue))
    (`self.K2_DestroyActor`)))

(fn `UserConstructionScript`)